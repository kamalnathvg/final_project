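; BP_Flare is a level-exit actor with a briefly shown beam that sends the VR player to Level_2.
; On BeginPlay it hides the beam, then uses delays to show it for a few seconds before hiding it again.
; ShowBeam and HideBeam toggle only DefaultSceneRoot's visibility, without propagating to children.
; Any overlap by a VRPawn opens Level_2, with no check on beam visibility.
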(event `self.ReceiveBeginPlay`
  ;[1 1 1] Show Beam When game starts
  (`self.HideBeam`)
  (`KismetSystemLibrary.Delay` 5.0)
  (`self.ShowBeam`)
  (`KismetSystemLibrary.Delay` 5.0)
  (`self.HideBeam`))

(event `self.ReceiveActorBeginOverlap`
  (params (OtherActor :type "Actor Object Reference"))
  ;[1 1 1] go to next level on complete
  (bind _asvrpawn (cast `/Game/VRTemplate/Blueprints/VRPawn` OtherActor))
  (`/Engine/EditorBlueprintResources/StandardMacros.IsValid` _asvrpawn
    (:`Is Valid`
      (`GameplayStatics.OpenLevel` "Level_2"))))

(fn `HideBeam`
  (`SceneComponent.SetVisibility` (`self.DefaultSceneRoot`) false false))

(fn `ShowBeam`
  (`SceneComponent.SetVisibility` (`self.DefaultSceneRoot`) true false))

(fn `UserConstructionScript`)